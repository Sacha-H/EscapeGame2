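; BP_RealDoorOpen is an interactive double door that swings open and closed once both key flags, Key1 and Key2, are true.
; Each successful Interact alternates through a FlipFlop between playing and reversing Timeline_DoorKey.
; The timeline's curve, scaled by AngleRotation, yaws the two door meshes in opposite directions.
; BeginPlay sets the play rate of RotationAngle, rather than Timeline_DoorKey, to the inverse of Duration.
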(event EventBeginPlay
  (Components|Timeline|SetPlayRate (Variables|Default|GetRotation%20Angle) (/ 1.0 (Variables|Default|GetDuration))))

(event Collision|EventActorBeginOverlap
  (params (OtherActor :type Actor%20Object%20Reference)))

(event EventTick
  (params (DeltaSeconds :type Float%20%28single-precision%29)))

(event EventInteract
  (if (and (Variables|Default|Getkey1) (Variables|Default|Getkey2))
    (Utilities|FlowControl|FlipFlop
      (:A
        (bind _anglerotation (Timeline|Timeline_DoorKey Play)
          (:Update
            (Transformation|SetRelativeRotation (Variables|Default|GetDoor_1_StaticMeshComponent0) (Math|Rotator|MakeRotator 0.0 0.0 (* (* _anglerotation (Variables|Default|GetAngleRotation)) -1.0)) false false)
            (Transformation|SetRelativeRotation (Variables|Default|GetDoor_2_StaticMeshComponent0) (Math|Rotator|MakeRotator 0.0 0.0 (* _anglerotation (Variables|Default|GetAngleRotation))) false false))))
      (:B
        (Timeline|Timeline_DoorKey Reverse)))))

(fn ConstructionScript)